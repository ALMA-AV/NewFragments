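; Interlude trigger actor that fades in its spotlights when the player character enters its box.
; A one-shot timeline drives the intensity of spotlights under LightContainer and their direct spotlight children.
; Overlap also starts a looping timer, cleared on exit, but its TimerSpawn event is empty.
; Disconnected logic would cycle through MeshesToSpawn, replacing a rotating object spawned in front of the actor.
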(event OnComponentBeginOverlap(Box)
  (params (OverlappedComponent :type Primitive%20Component%20Object%20Reference) (OtherActor :type Actor%20Object%20Reference) (OtherComp :type Primitive%20Component%20Object%20Reference) (OtherBodyIndex :type Integer) (bFromSweep :type Boolean) (SweepResult :type Hit%20Result%20Structure%20%28by%20ref%29))
  (Utilities|Casting|CastToBP_Fragements_Character OtherActor)
  (bind _returnvalue (Utilities|Time|SetTimerbyEvent (delegate Custom|TimerSpawn) 1e+01 true))
  (Variables|Default|SetSppawnerTimer _returnvalue)
  (if (not (Variables|Default|GetLightsOn))
    (bind _lightintensity (Timeline|Timeline_0 PlayFromStart)
      (:Update
        (for _array_element (Components|GetChildrenComponents (Variables|Default|GetLightContainer) false)
          (bind _asspot_light_component (Utilities|Casting|CastToSpotLightComponent _array_element))
          (Rendering|Components|Light|SetIntensity _asspot_light_component _lightintensity)
          (for _array_element_2 (Components|GetChildrenComponents _array_element false)
            (bind _asspot_light_component_2 (Utilities|Casting|CastToSpotLightComponent _array_element_2))
            (Rendering|Components|Light|SetIntensity _asspot_light_component_2 _lightintensity))))
      (:Finished
        (Variables|Default|SetLightsOn true)))))

(event OnComponentEndOverlap(Box)
  (params (OverlappedComponent :type Primitive%20Component%20Object%20Reference) (OtherActor :type Actor%20Object%20Reference) (OtherComp :type Primitive%20Component%20Object%20Reference) (OtherBodyIndex :type Integer))
  (Utilities|Casting|CastToBP_Fragements_Character OtherActor)
  (Utilities|Time|ClearandInvalidateTimerbyHandle (Variables|Default|GetSppawnerTimer)))

(event Custom|TimerSpawn)

(event EventBeginPlay)

(event Collision|EventActorBeginOverlap
  (params (OtherActor :type Actor%20Object%20Reference)))

(event EventTick
  (params (DeltaSeconds :type Float%20%28single-precision%29)))

(fn ConstructionScript)