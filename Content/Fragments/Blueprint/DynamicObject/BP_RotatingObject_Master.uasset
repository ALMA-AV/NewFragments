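; BP_RotatingObject_Master is a dynamic object Blueprint that continuously spins a static mesh around its yaw axis.
; The construction script assigns the Mesh variable to the StaticMesh component.
; Each Tick adds RotationSpeed to the component's relative yaw and zeroes pitch and roll, without delta-time scaling, so spin rate depends on frame rate.
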(event EventBeginPlay)

(event Collision|EventActorBeginOverlap
  (params (OtherActor :type Actor%20Object%20Reference)))

(event EventTick
  (params (DeltaSeconds :type Float%20%28single-precision%29))
  (Transformation|SetRelativeRotation (Variables|Default|GetStaticMesh) (Math|Rotator|MakeRotator 0.0 0.0 (+ (.yaw (Variables|/Script/Engine.SceneComponent|GetRelativeRotation (Variables|Default|GetStaticMesh))) (* 1.0 (Variables|Default|GetRotationSpeed)))) false false))

(fn ConstructionScript
  (Components|StaticMesh|SetStaticMesh (Variables|Default|GetStaticMesh) (Variables|Default|GetMesh)))