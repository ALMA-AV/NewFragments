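; Player controller for Fragments that flies BP_Fragements_Character and lets an external OSC sender drive the scene live.
; An OSC server routes messages by address to movement variables, sun, fog, post-process, environment material modes, subtitles and titles.
; Input axes drive flight with speed modifiers, while Tick applies smoothed rotation or aims at a locked point.
; Saved drop points support timeline-lerped recall, and texture mode switches use delays, with a glitch effect for some.
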(event Custom|OSCMessageReceived
  (params (Message :type OSC%20Message%20Structure%20%28by%20ref%29) (IPAddress :type String) (Port :type Integer))
  (bind _returnvalue (Class|OSCManager|GetOSCMessageAddress Message))
  (bind _returnvalue_2 (Class|OSCManager|GetOSCAddressFullPath _returnvalue))
  (switch string _returnvalue_2
    (:/Movement/Direction
      (bind _value (Class|OSCManager|GetFloat Message 1))
      (Variables|Default|SetForwardThruster _value)
      (bind _value_2 (Class|OSCManager|GetFloat Message))
      (Variables|Default|SetSideThruster _value_2))
    (:/Movement/Vertical
      (bind _value_3 (Class|OSCManager|GetFloat Message))
      (Variables|Default|SetVerticalThruster _value_3))
    (:/Movement/Speed
      (bind _value_4 (Class|OSCManager|GetFloat Message))
      (Variables|Default|SetSpeedScalar _value_4))
    (:/Movement/Orientation
      (bind _value_5 (Class|OSCManager|GetFloat Message))
      (Variables|Default|SetXRotation _value_5)
      (bind _value_6 (Class|OSCManager|GetFloat Message 1))
      (Variables|Default|SetYRotation _value_6))
    (:/Movement/Lock
      (bind _value_7 (Class|OSCManager|GetFloat Message))
      (if (== _value_7 1.0)
        (Variables|Default|SetIsLockedOnPoint? true)
        (CallFunction|SetLockonPoint)
        (else
          (Variables|Default|SetIsLockedOnPoint? false))))
    (:/Sun/Intensity
      (bind _value_8 (Class|OSCManager|GetFloat Message))
      (CallFunction|SetSunIntensity (* _value_8 1e+01)))
    (:/Sun/Yaw
      (bind _value_9 (Class|OSCManager|GetFloat Message))
      (CallFunction|SetSunPosition (* _value_9 3.6e+02)))
    (:/Sun/Temperature
      (bind _value_10 (Class|OSCManager|GetFloat Message))
      (CallFunction|SetSunTemperature (+ (* _value_10 1e+04) 2e+03)))
    (:/Fog/Intensity
      (bind _value_11 (Class|OSCManager|GetFloat Message))
      (CallFunction|SetFogIntensity (* (Math|Float|Power _value_11 2.0) 0.5)))
    (:/Texture/Mode
      (bind _value_12 (Class|OSCManager|GetFloat Message))
      (switch int (Math|Float|Truncate _value_12)
        (:0
          (CallFunction|SetPostProcessIntensity 1.0)
          (Utilities|FlowControl|Delay 1.0)
          (CallFunction|SetTextureasPolygon)
          (CallFunction|SetFogIntensity 0.08))
        (:1
          (CallFunction|SetPostProcessIntensity 1.0)
          (Utilities|FlowControl|Delay 1.0)
          (CallFunction|SetTextureasPoints)
          (CallFunction|SetFogIntensity 0.0))
        (:2
          (CallFunction|SetPostProcessIntensity 0.0)
          (Utilities|FlowControl|Delay 1.0)
          (CallFunction|SetTextureasGrid)
          (CallFunction|SetFogIntensity 0.0)))
      (CallFunction|SetPostProcessIntensity 0.0))
    (:/Camera/BlurKM
      (bind _value_13 (Class|OSCManager|GetFloat Message))
      (CallFunction|SetFocalKM (* (Math|Float|Power _value_13 2.0) 1.0)))
    (:/Camera/Contrast
      (bind _value_14 (Class|OSCManager|GetFloat Message))
      (CallFunction|SetContrast (* _value_14 2.0)))
    (:/Texture/Glow
      (bind _value_15 (Class|OSCManager|GetFloat Message))
      (CallFunction|SetTextureGlow (* (Math|Float|Power _value_15 2.0) 5e+01)))
    (:/DropPoint
      (bind _value_16 (Class|OSCManager|GetFloat Message))
      ;[1 1 1] set fast recall for ACT II
      (if (> _value_16 17.0)
        (Variables|DropPoints|SetRecallSpeed 6.0)
        (else
          (Variables|DropPoints|SetRecallSpeed 1.0)))
      (Development|PrintString "Hello")
      (if (!= _value_16 0.0)
        (if (Variables|DropPoints|GetSavingDropPoint)
          (CallFunction|SaveNewDropPoint (Math|Float|Truncate _value_16))
          (else
            (CallFunction|RecalltoDropPoint (Math|Float|Truncate _value_16))
            (if (== (Math|Float|Truncate _value_16) 16)
              (bind _returnvalue_3 (Actor|GetActorOfClass "/Game/Fragments/Blueprint/DynamicObject/BP_InterludeSpawner.BP_InterludeSpawner_C"))
              (Development|SetHiddeninGame (Variables|/Game/Fragments/Blueprint/DynamicObject/BP_InterludeSpawner.BP_InterludeSpawner_C|GetBP_NY_1 _returnvalue_3) false false)
              (else
                (Utilities|FlowControl|Delay 1e+01)
                (bind _returnvalue_4 (Actor|GetActorOfClass "/Game/Fragments/Blueprint/DynamicObject/BP_InterludeSpawner.BP_InterludeSpawner_C"))
                (Development|SetHiddeninGame (Variables|/Game/Fragments/Blueprint/DynamicObject/BP_InterludeSpawner.BP_InterludeSpawner_C|GetBP_NY_1 _returnvalue_4) true false)))))))
    (:/DropPoint/Save
      (bind _value_17 (Class|OSCManager|GetFloat Message))
      (if (== _value_17 1.0)
        (Variables|DropPoints|SetSavingDropPoint true)
        (else
          (Variables|DropPoints|SetSavingDropPoint false))))
    (:/DropPoint/Speed
      (bind _value_18 (Class|OSCManager|GetFloat Message))
      (Variables|DropPoints|SetRecallSpeed (+ (* (Math|Float|Power _value_18 2.0) 3e+01) 1.0)))
    (:/Subtitle
      (bind _value_19 (Class|OSCManager|GetFloat Message))
      (if (== _value_19 1.0)
        (Default|PlaySubtitle1 (Variables|Default|GetSubtitleWidget))
        (elif (== _value_19 2.0)
          (Default|PlaySubtitle2 (Variables|Default|GetSubtitleWidget)))))
    (:/Titles
      (bind _value_20 (Class|OSCManager|GetInt32 Message))
      (Default|SetTitles (Variables|Default|GetTitlesWidget) _value_20))))

(event Custom|RecalltoDropPoint
  (params (RecallDropPointIndex :type Integer))
  (bind _characterref (Variables|Default|GetCharacterRef))
  (Variables|DropPoints|SetRecall%20Drop%20Point%20Index RecallDropPointIndex)
  (Variables|DropPoints|SetIsRecalling? true)
  (Variables|Default|SetCanMove? false)
  (Variables|DropPoints|SetSaveCharacterLocation (Transformation|GetActorLocation _characterref))
  (Variables|DropPoints|SetSaveCharacterRotation (Transformation|GetActorRotation _characterref))
  (bind _lerpamount (Timeline|RecallTimeline PlayFromStart)
    (:Update
      (Utilities|FlowControl|Sequence
        (:then_0
          (Transformation|SetActorLocation (Variables|Default|GetCharacterRef) (Math|Vector|Lerp(Vector) (Variables|DropPoints|GetSaveCharacterLocation) (Utilities|Array|Get(acopy) (Variables|DropPoints|GetDropPoints) (Variables|DropPoints|GetRecall%20Drop%20Point%20Index)) (* _lerpamount (Variables|DropPoints|GetRecallSpeed))) false false)
          (if (>= (* _lerpamount (Variables|DropPoints|GetRecallSpeed)) 1.0)
            (Utilities|FlowControl|Sequence
              (:then_0
                (Timeline|RecallTimeline Stop))
              (:then_1
                (Variables|DropPoints|SetIsRecalling? false)
                (Variables|Default|SetCanMove? true)))))
        (:then_1
          (Pawn|SetControlRotation (Math|Rotator|Lerp(Rotator) (Variables|DropPoints|GetSaveCharacterRotation) (Utilities|Array|Get(acopy) (Variables|DropPoints|GetDropPointRotation) (Variables|DropPoints|GetRecall%20Drop%20Point%20Index)) (* _lerpamount (Variables|DropPoints|GetRecallSpeed)) true)))))
    (:Finished
      (Variables|DropPoints|SetIsRecalling? false)
      (Variables|Default|SetCanMove? true))))

(event EventBeginPlay
  (bind _asbp_fragements_character (Utilities|Casting|CastToBP_Fragements_Character (Pawn|GetControlledPawn))
    (:then
      (Variables|Default|SetCharacterRef _asbp_fragements_character)
      (bind _returnvalue (Class|OSCManager|CreateOSCServer "0.0.0.0" 5400 false true "" 0))
      (bind _output_get (Variables|Default|SetOSCServer _returnvalue))
      (Development|PrintString (Utilities|GetDisplayName _output_get))
      (EventDispatchers|BindEventtoOnOscMessageReceived _output_get (delegate Custom|OSCMessageReceived))
      (bind _returnvalue_2 (Actor|GetActorOfClass "/Script/Engine.PostProcessVolume"))
      (Variables|Default|SetPostProcessRef _returnvalue_2)
      (bind _returnvalue_3 (Rendering|Material|CreateDynamicMaterialInstance "/Game/Blueprints/Materials/MI_PostProcessGlitch.MI_PostProcessGlitch" "None" "None" :!class /Script/Engine.KismetMaterialLibrary))
      (bind _output_get_2 (Variables|Default|SetPostProcessMaterial _returnvalue_3))
      (Rendering|Material|SetMaterial (Variables|/Script/Engine.Brush|GetBrushComponent (Variables|Default|GetPostProcessRef)) 0 _output_get_2)
      (CallFunction|SetPostProcessIntensity 0.0)
      (bind _returnvalue_4 (UserInterface|CreateWidget "/Game/Fragments/UI/W_Subtitle.W_Subtitle_C"))
      (Variables|Default|SetSubtitleWidget _returnvalue_4)
      (UserInterface|Viewport|AddtoViewport _returnvalue_4 0)
      (bind _returnvalue_5 (UserInterface|CreateWidget "/Game/Fragments/UI/W_Titles.W_Titles_C"))
      (Variables|Default|SetTitlesWidget _returnvalue_5)
      (UserInterface|Viewport|AddtoViewport _returnvalue_5 0))
    (:CastFailed
      (Development|PrintString "**SHOULD NEVER HAPPEN** Not BP_Fragment_Character"))))

(event EventTick
  (params (DeltaSeconds :type Float%20%28single-precision%29))
  (bind _returnvalue (Pawn|GetControlRotation :!class /Script/Engine.Controller))
  ;[1 1 1] Rotation
  (Variables|Default|SetDelta%20Seconds DeltaSeconds)
  (if (Variables|Default|GetIsLockedOnPoint?)
    (CallFunction|SetRotationonLockPoint)
    (else
      (Pawn|SetControlRotation (Math|Rotator|MakeRotator 0.0 (+ (.pitch _returnvalue) (Class|KismetMathLibrary|WeightedMovingAverageFloat (Variables|Default|GetPitchToAdd) (Variables|Default|GetPreviousPitch) 0.05)) (+ (.yaw _returnvalue) (Class|KismetMathLibrary|WeightedMovingAverageFloat (Variables|Default|GetYawToAdd) (Variables|Default|GetPreviousYaw) 0.05))))
      (Variables|Default|SetPreviousPitch (Variables|Default|GetPitchToAdd))
      (Variables|Default|SetPreviousYaw (Variables|Default|GetYawToAdd)))))

(event Input|ActionEvents|InputActionKeepRotationToggle
  (params (Key :type Key%20Structure :default "None"))
  (:Pressed
    (Variables|Default|SetMaintainRotation true))
  (:Released
    (Variables|Default|SetMaintainRotation false)))

(event Input|ActionEvents|InputActionSetDropPoint2
  (params (Key :type Key%20Structure :default "None"))
  ;[1 1 1] DropPoint2
  (:Pressed
    (CallFunction|SaveNewDropPoint 2)))

(event Input|ActionEvents|InputActionRecallDropPoint2
  (params (Key :type Key%20Structure :default "None"))
  ;[1 1 1] DropPoint2
  (:Pressed
    (Variables|DropPoints|SetRecallSpeed 6.0)
    (CallFunction|RecalltoDropPoint 2)))

(event Input|ActionEvents|InputActionSpeedBoost
  (params (Key :type Key%20Structure :default "None"))
  ;[1 1 1] Speed Modifier
  (:Pressed
    (if (!= (Variables|Default|GetSpeedBoost) 2.0)
      (Variables|Default|SetSpeedBoost 1e+01) ; speed value is actually clamped to 1, just to ensure we boost it to the max
      (else
        (Variables|Default|SetSpeedBoost 1.0)))))

(event Input|ActionEvents|InputActionSpeedSlowMo
  (params (Key :type Key%20Structure :default "None"))
  ;[1 1 1] Speed Modifier
  (:Pressed
    (if (!= (Variables|Default|GetSpeedBoost) 0.25)
      (Variables|Default|SetSpeedBoost 0.25)
      (else
        (Variables|Default|SetSpeedBoost 1.0)))))

(event Input|AxisEvents|InputAxisMoveForwardAxis
  (params (AxisValue :type Float%20%28single-precision%29))
  (if (Variables|Default|GetCanMove?)
    (Pawn|Input|AddMovementInput (Variables|Default|GetCharacterRef) (Math|Vector|GetForwardVector (Variables|/Script/Engine.Character|GetCapsuleComponent (Variables|Default|GetCharacterRef))) AxisValue false)))

(event Input|AxisEvents|InputAxisMovesideAxis
  (params (AxisValue :type Float%20%28single-precision%29))
  (if (Variables|Default|GetCanMove?)
    (Pawn|Input|AddMovementInput (Variables|Default|GetCharacterRef) (Math|Vector|GetRightVector (Variables|/Script/Engine.Character|GetCapsuleComponent (Variables|Default|GetCharacterRef))) AxisValue false)))

(event Input|AxisEvents|InputAxisMoveUpAxis
  (params (AxisValue :type Float%20%28single-precision%29))
  (if (Variables|Default|GetCanMove?)
    (Pawn|Input|AddMovementInput (Variables|Default|GetCharacterRef) (Math|Vector|GetUpVector (Variables|/Script/Engine.Character|GetCapsuleComponent (Variables|Default|GetCharacterRef))) AxisValue false)))

(event Input|AxisEvents|InputAxisControllerForwardMovement
  (params (AxisValue :type Float%20%28single-precision%29))
  (if (Variables|Default|GetCanMove?)
    (Pawn|Input|AddMovementInput (Variables|Default|GetCharacterRef) (Math|Vector|GetForwardVector (Variables|/Script/Engine.Character|GetCapsuleComponent (Variables|Default|GetCharacterRef))) (* (Variables|Default|GetSpeedBoost) (* (Variables|Default|GetSpeedScalar) AxisValue)) false)))

(event Input|AxisEvents|InputAxisLookUp
  (params (AxisValue :type Float%20%28single-precision%29))
  (bind _returnvalue (Pawn|GetControlRotation :!class /Script/Engine.Controller))
  (bind _turnrate (Variables|Default|GetturnRate))
  (if (and (Variables|Default|GetCanMove?) (not (Variables|Default|GetIsLockedOnPoint?)))
    (Pawn|SetControlRotation (Math|Rotator|MakeRotator 0.0 (+ (.pitch _returnvalue) (* _turnrate AxisValue)) (+ (.yaw _returnvalue) (* _turnrate (Input|AxisValues|GetLookSide)))))))

(event Input|AxisEvents|InputAxisControllerSideMovement
  (params (AxisValue :type Float%20%28single-precision%29))
  (if (Variables|Default|GetCanMove?)
    (Pawn|Input|AddMovementInput (Variables|Default|GetCharacterRef) (Math|Vector|GetRightVector (Variables|/Script/Engine.Character|GetCapsuleComponent (Variables|Default|GetCharacterRef))) (* (Variables|Default|GetSpeedBoost) (* (Variables|Default|GetSpeedScalar) AxisValue)) false)))

(event Input|AxisEvents|InputAxisControllerupMovement
  (params (AxisValue :type Float%20%28single-precision%29))
  (if (Variables|Default|GetCanMove?)
    (Pawn|Input|AddMovementInput (Variables|Default|GetCharacterRef) (Math|Vector|GetUpVector (Variables|/Script/Engine.Character|GetCapsuleComponent (Variables|Default|GetCharacterRef))) (* (Variables|Default|GetSpeedBoost) (* (Variables|Default|GetSpeedScalar) AxisValue)) false)))

(event Input|AxisEvents|InputAxisControllerLookup
  (params (AxisValue :type Float%20%28single-precision%29))
  (bind _speedboost (Variables|Default|GetSpeedBoost))
  (bind _turnrate (Variables|Default|GetturnRate))
  (bind _returnvalue (Math|Float|Clamp(Float) _speedboost 1.0 2.0))
  (if (and (Variables|Default|GetCanMove?) (not (Variables|Default|GetIsLockedOnPoint?)))
    (if (not (Variables|Default|GetMaintainRotation))
      (Variables|Default|SetPitchToAdd (* (* _turnrate AxisValue) _returnvalue))
      (Variables|Default|SetYawToAdd (* (* _turnrate (Input|AxisValues|GetControllerLookSide)) _returnvalue)))))

(event Input|KeyboardEvents|R
  (params (Key :type Key%20Structure :default "None"))
  ;[1 1 1] Save screenshot
  (:Pressed
    (Development|ExecuteConsoleCommand "shot" 0)
    (Development|PrintString "screenshot saved")))

(event Input|MouseEvents|RightMouseButton
  (params (Key :type Key%20Structure :default "None"))
  (:Pressed
    (Variables|Default|SetIsLockedOnPoint? true)
    (CallFunction|SetLockonPoint))
  (:Released
    (Variables|Default|SetIsLockedOnPoint? false)))

(event Input|KeyboardEvents|P
  (params (Key :type Key%20Structure :default "None"))
  (bind _characterref (Variables|Default|GetCharacterRef))
  (bind _returnvalue (Transformation|GetActorRotation _characterref))
  ;[1 1 1] P - print position
  (:Pressed
    (Development|PrintString (Utilities|String|ToString(Text) (Utilities|Text|FormatText "Position: {position} --  Rotation: Y={yaw}  P={pitch}  R={roll}" (Utilities|String|ToString(Vector) (Transformation|GetActorLocation (Variables|Default|GetCharacterRef))) (.roll _returnvalue) (.pitch _returnvalue) (.yaw _returnvalue))) true true "(R=0.000000,G=0.660000,B=1.000000,A=1.000000)" 6e+01)))

(event Input|KeyboardEvents|1
  (params (Key :type Key%20Structure :default "None"))
  ;[1 1 1] keyboard shortcuts for testing
  (:Pressed
    (Utilities|FlowControl|FlipFlop
      (:A
        (CallFunction|SetSunIntensity 0.0))
      (:B
        (CallFunction|SetSunIntensity 0.35)))))

(event Input|KeyboardEvents|2
  (params (Key :type Key%20Structure :default "None"))
  ;[1 1 1] keyboard shortcuts for testing
  (:Pressed
    (CallFunction|RecalltoDropPoint 16)
    (bind _returnvalue (Actor|GetActorOfClass "/Game/Fragments/Blueprint/DynamicObject/BP_InterludeSpawner.BP_InterludeSpawner_C"))
    (Development|SetHiddeninGame (Variables|/Game/Fragments/Blueprint/DynamicObject/BP_InterludeSpawner.BP_InterludeSpawner_C|GetBP_NY_1 _returnvalue) false false)))

(event Input|GamepadEvents|GamepadRightShoulder
  (params (Key :type Key%20Structure :default "None"))
  (bind _returnvalue (Game|GetPlayerCharacter 0))
  (:Pressed
    (bind _asbp_fragements_character (Utilities|Casting|CastToBP_Fragements_Character _returnvalue))
    (Effects|Components|ParticleSystem|SetFloatParameter (Variables|/Game/Fragments/Blueprint/BP_Fragements_Character.BP_Fragements_Character_C|GetNS_DistanceFieldParticles _asbp_fragements_character) "SpawnRate" 1e+04))
  (:Released
    (bind _asbp_fragements_character_2 (Utilities|Casting|CastToBP_Fragements_Character _returnvalue))
    (Effects|Components|ParticleSystem|SetFloatParameter (Variables|/Game/Fragments/Blueprint/BP_Fragements_Character.BP_Fragements_Character_C|GetNS_DistanceFieldParticles _asbp_fragements_character_2) "SpawnRate" 0.0)))

(event Input|KeyboardEvents|3
  (params (Key :type Key%20Structure :default "None"))
  ;[1 1 1] keyboard shortcuts for testing
  (:Pressed
    (Utilities|FlowControl|FlipFlop
      (:A
        (CallFunction|SetFogIntensity 0.0))
      (:B
        (CallFunction|SetFogIntensity 0.08)))))

(event Input|KeyboardEvents|4
  (params (Key :type Key%20Structure :default "None"))
  ;[1 1 1] keyboard shortcuts for testing
  (:Pressed
    (Variables|DropPoints|SetRecallSpeed 6.0)))

(fn ConstructionScript)

(fn SaveNewDropPoint
  (params (Index :type Integer))
  (bind _characterref (Variables|Default|GetCharacterRef))
  (Utilities|Array|SetArrayElem (Variables|DropPoints|GetDropPoints) Index (Transformation|GetActorLocation _characterref) true)
  (Utilities|Array|SetArrayElem (Variables|DropPoints|GetDropPointRotation) Index (Transformation|GetActorRotation _characterref) true)
  (return))

(fn SetSunPosition
  (params (New%20Rotation%20Z%20%28Yaw%29 :type Float%20%28single-precision%29))
  (bind _returnvalue (Actor|GetActorOfClass "/Script/Engine.DirectionalLight"))
  (Transformation|SetActorRotation _returnvalue (Math|Rotator|MakeRotator (.roll (Transformation|GetActorRotation _returnvalue)) (.pitch (Transformation|GetActorRotation _returnvalue)) New%20Rotation%20Z%20%28Yaw%29))
  (return))

(fn SetSunIntensity
  (params (NewIntensity :type Float%20%28single-precision%29))
  (bind _returnvalue (Actor|GetActorOfClass "/Script/Engine.DirectionalLight"))
  (Rendering|Components|Light|SetIntensity (Variables|/Script/Engine.Light|GetLightComponent _returnvalue) NewIntensity)
  (return))

(fn SetSunTemperature
  (params (NewTemperature :type Float%20%28single-precision%29))
  (bind _returnvalue (Actor|GetActorOfClass "/Script/Engine.DirectionalLight"))
  (Class|LightComponent|SetTemperature (Variables|/Script/Engine.Light|GetLightComponent _returnvalue) NewTemperature)
  (return))

(fn SetFogIntensity
  (params (NewDensity :type Float%20%28single-precision%29))
  (bind _returnvalue (Actor|GetActorOfClass "/Script/Engine.ExponentialHeightFog"))
  (Class|ExponentialHeightFogComponent|SetFogDensity (Variables|/Script/Engine.ExponentialHeightFog|GetComponent _returnvalue) NewDensity)
  (return))

(fn SetLockonPoint
  (bind _characterref (Variables|Default|GetCharacterRef))
  (Variables|Default|SetLockLocation (+ (Transformation|GetActorLocation _characterref) (* (Math|Vector|GetForwardVector (Variables|/Script/Engine.Character|GetCapsuleComponent _characterref)) (Variables|Default|GetLockOnDistance))))
  (return))

(fn SetRotationonLockPoint
  (Pawn|SetControlRotation (Math|Rotator|FindLookatRotation (Transformation|GetActorLocation (Variables|Default|GetCharacterRef)) (Variables|Default|GetLockLocation)))
  (return))

(fn SetTextureasPoints
  (bind _outactors (Actor|GetAllActorsOfClass "/Game/Fragments/Blueprint/EnviromentObjects/BP_EnvironmentObjectMaster.BP_EnvironmentObjectMaster_C"))
  (for _array_element _outactors
    (Rendering|Material|SetScalarParameterValue (Variables|/Game/Fragments/Blueprint/EnviromentObjects/BP_EnvironmentObjectMaster.BP_EnvironmentObjectMaster_C|GetDynamicMaterialInstance _array_element) "MaskSelect" 0.0 :!class /Script/Engine.MaterialInstanceDynamic)
    (Rendering|Material|SetScalarParameterValue (Variables|/Game/Fragments/Blueprint/EnviromentObjects/BP_EnvironmentObjectMaster.BP_EnvironmentObjectMaster_C|GetDynamicMaterialInstance _array_element) "MaskOn" 1.0 :!class /Script/Engine.MaterialInstanceDynamic))
  (return))

(fn SetTextureasGrid
  (bind _outactors (Actor|GetAllActorsOfClass "/Game/Fragments/Blueprint/EnviromentObjects/BP_EnvironmentObjectMaster.BP_EnvironmentObjectMaster_C"))
  (for _array_element _outactors
    (Rendering|Material|SetScalarParameterValue (Variables|/Game/Fragments/Blueprint/EnviromentObjects/BP_EnvironmentObjectMaster.BP_EnvironmentObjectMaster_C|GetDynamicMaterialInstance _array_element) "MaskSelect" 1.0 :!class /Script/Engine.MaterialInstanceDynamic)
    (Rendering|Material|SetScalarParameterValue (Variables|/Game/Fragments/Blueprint/EnviromentObjects/BP_EnvironmentObjectMaster.BP_EnvironmentObjectMaster_C|GetDynamicMaterialInstance _array_element) "MaskOn" 1.0 :!class /Script/Engine.MaterialInstanceDynamic))
  (return))

(fn SetTextureasPolygon
  (bind _outactors (Actor|GetAllActorsOfClass "/Game/Fragments/Blueprint/EnviromentObjects/BP_EnvironmentObjectMaster.BP_EnvironmentObjectMaster_C"))
  (for _array_element _outactors
    (Rendering|Material|SetScalarParameterValue (Variables|/Game/Fragments/Blueprint/EnviromentObjects/BP_EnvironmentObjectMaster.BP_EnvironmentObjectMaster_C|GetDynamicMaterialInstance _array_element) "MaskSelect" 0.0 :!class /Script/Engine.MaterialInstanceDynamic)
    (Rendering|Material|SetScalarParameterValue (Variables|/Game/Fragments/Blueprint/EnviromentObjects/BP_EnvironmentObjectMaster.BP_EnvironmentObjectMaster_C|GetDynamicMaterialInstance _array_element) "MaskOn" 0.0 :!class /Script/Engine.MaterialInstanceDynamic))
  (return))

(fn SetFocalKM
  (params (Depth%20Blur%20km%20for%2050%25 :type Float%20%28single-precision%29))
  (bind _returnvalue (Actor|GetActorOfClass "/Script/Engine.PostProcessVolume"))
  (Utilities|Struct|SetmembersinPostProcessSettings (Variables|/Script/Engine.PostProcessVolume|GetSettings _returnvalue) Depth%20Blur%20km%20for%2050%25)
  (return))

(fn SetContrast
  (params (Contrast :type Float%20%28single-precision%29))
  (bind _returnvalue (Actor|GetActorOfClass "/Script/Engine.PostProcessVolume"))
  (Utilities|Struct|SetmembersinPostProcessSettings (Variables|/Script/Engine.PostProcessVolume|GetSettings _returnvalue) (Math|Vector4|MakeVector4 Contrast Contrast Contrast Contrast))
  (return))

(fn SetTextureGlow
  (params (Value :type Float%20%28single-precision%29))
  (bind _outactors (Actor|GetAllActorsOfClass "/Game/Fragments/Blueprint/EnviromentObjects/BP_EnvironmentObjectMaster.BP_EnvironmentObjectMaster_C"))
  (for _array_element _outactors
    (Rendering|Material|SetScalarParameterValue (Variables|/Game/Fragments/Blueprint/EnviromentObjects/BP_EnvironmentObjectMaster.BP_EnvironmentObjectMaster_C|GetDynamicMaterialInstance _array_element) "Glow" Value :!class /Script/Engine.MaterialInstanceDynamic))
  (return))

(fn SetPostProcessIntensity
  (params (Intensity :type Float%20%28single-precision%29))
  (Utilities|Struct|SetmembersinPostProcessSettings (Variables|/Script/Engine.PostProcessVolume|GetSettings (Variables|Default|GetPostProcessRef)) (Utilities|Struct|MakeWeightedBlendables (Utilities|Array|MakeArray (Utilities|Struct|MakeWeightedBlendable Intensity (Variables|Default|GetPostProcessMaterial)))))
  (return))