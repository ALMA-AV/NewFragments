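; BP_EnvironmentObjectMaster is a configurable base actor for environment props with a per-instance mesh, textures and tiling.
; The construction script assigns MeshToAdd to ObjectMesh, so the chosen mesh shows in the editor.
; On BeginPlay it creates a dynamic instance of MI_ObjectsMaster on slot 0 and applies the base texture, normal map and tiling, so material overrides appear only at runtime.
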(event EventBeginPlay
  (bind _objectmesh (Variables|Default|GetObjectMesh))
  (bind _returnvalue (Rendering|Material|CreateDynamicMaterialInstance _objectmesh 0 "/Game/Fragments/Geometry/MI_ObjectsMaster.MI_ObjectsMaster" "None" :!class /Script/Engine.PrimitiveComponent))
  (bind _output_get (Variables|Default|SetDynamicMaterialInstance _returnvalue))
  (Rendering|Material|SetTextureParameterValue _output_get "BaseTexture" (Variables|Default|GetTexture))
  (Rendering|Material|SetTextureParameterValue _output_get "NormalMap" (Variables|Default|GetNormalMap))
  (Rendering|Material|SetMaterial _objectmesh 0 (Variables|Default|GetDynamicMaterialInstance))
  (Rendering|Material|SetScalarParameterValue (Variables|Default|GetDynamicMaterialInstance) "Tiling" (Variables|Default|GetTiling) :!class /Script/Engine.MaterialInstanceDynamic))

(event Collision|EventActorBeginOverlap
  (params (OtherActor :type Actor%20Object%20Reference)))

(event EventTick
  (params (DeltaSeconds :type Float%20%28single-precision%29)))

(fn ConstructionScript
  (Components|StaticMesh|SetStaticMesh (Variables|Default|GetObjectMesh) (Variables|Default|GetMeshToAdd)))